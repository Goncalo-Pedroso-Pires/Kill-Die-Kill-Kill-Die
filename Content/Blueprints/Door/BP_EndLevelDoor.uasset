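; End-of-level door that moves the player on to the next level once the current one is cleared.
; It caches BP_FirstPersonGameMode on BeginPlay, and when the player pawn overlaps its box it checks that game mode's AllSpawsRemoved flag.
; If the flag is set, a hardcoded chain of level-name checks picks the destination: the tutorial leads into Level_1, and the three numbered levels cycle back to the first.
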(event `self.ReceiveBeginPlay`
  (bind _asbp_first_person_game_mode (cast `/Game/FirstPerson/Blueprints/BP_FirstPersonGameMode` (`GameplayStatics.GetGameMode`)))
  (set `self.GameMode` _asbp_first_person_game_mode))

(event `self.Box.OnComponentBeginOverlap`
  (params (OverlappedComponent :type "PrimitiveComponent Object Reference") (OtherActor :type "Actor Object Reference") (OtherComp :type "PrimitiveComponent Object Reference") (OtherBodyIndex :type Integer) (bFromSweep :type Boolean) (SweepResult :type "HitResult Structure (by ref)"))
  (if (== OtherActor (`GameplayStatics.GetPlayerPawn` 0))
    (if (`/Game/FirstPerson/Blueprints/BP_FirstPersonGameMode.AllSpawsRemoved?` (`self.GameMode`))
      (bind _returnvalue (`GameplayStatics.GetCurrentLevelName` true))
      (if (`KismetStringLibrary.EqualEqual_StrStr` _returnvalue "Level_1")
        (`GameplayStatics.OpenLevel` "Level_2")
        (elif (`KismetStringLibrary.EqualEqual_StrStr` _returnvalue "Level_2")
          (`GameplayStatics.OpenLevel` "Level_3")
          (elif (`KismetStringLibrary.EqualEqual_StrStr` _returnvalue "Level_3")
            (`GameplayStatics.OpenLevel` "Level_1")
            (elif (`KismetStringLibrary.EqualEqual_StrStr` _returnvalue "tutorial")
              (`GameplayStatics.OpenLevel` "Level_1"))))))))

(fn `UserConstructionScript`)