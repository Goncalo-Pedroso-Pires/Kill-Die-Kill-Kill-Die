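; Base enemy Blueprint that chases the player, deals contact damage and registers itself with the first-person game mode's enemy count.
; Tick reissues AIMoveTo toward the player's location, while sphere overlap starts a self-repeating, cooldown-gated attack that continues as long as the player stays inside.
; Incoming damage plays hurt or death sounds; on death it calls the empty DropWeapon event if rare, unregisters and destroys itself.
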(event `self.ReceiveBeginPlay`
  (set `self.Health` (`self.MaxHealth`))
  (bind _asbp_first_person_character (cast `/Game/Blueprints/BP_FirstPersonCharacter` (`GameplayStatics.GetPlayerPawn` 0)))
  (set `self.MainCharather` _asbp_first_person_character)
  (bind _asbp_first_person_game_mode (cast `/Game/FirstPerson/Blueprints/BP_FirstPersonGameMode` (`GameplayStatics.GetGameMode`)))
  (bind _output_get (set `self.As BP First Person Game Mode` _asbp_first_person_game_mode))
  (`/Game/FirstPerson/Blueprints/BP_FirstPersonGameMode.ADDEnemies` _output_get))

(event `self.ReceiveTick`
  (params (DeltaSeconds :type "Float (single-precision)"))
  (`|AIMoveTo` self (`self.K2_GetActorLocation` (`GameplayStatics.GetPlayerPawn` 0)) null))

(event `/Game/Blueprints/Enemies/Damageable.DamageTaken`
  (params (Damage :type "Float (double-precision)"))
  (bind _returnvalue (`SceneComponent.K2_GetComponentLocation` (`self.Mesh`)))
  (bind _returnvalue_2 (- (`self.Health`) Damage))
  (`GameplayStatics.PlaySoundAtLocation` "/Game/Audio/SFX/Sound_effects/Enemies/enemyHURT.enemyHURT" _returnvalue (struct) 1.0 1.0 0.0 null null null null)
  (`KismetSystemLibrary.PrintString` (`KismetStringLibrary.Conv_DoubleToString` _returnvalue_2))
  (bind _output_get (set `self.Health` _returnvalue_2))
  (if (<= _output_get 0.0)
    (`GameplayStatics.PlaySoundAtLocation` "/Game/Audio/SFX/Sound_effects/Enemies/EnemyDEATH.EnemyDEATH" _returnvalue (struct) 1.0 1.0 0.0 null null null null)
    (if (`self.isRare`)
      (`self.DropWeapon`))
    (`/Game/FirstPerson/Blueprints/BP_FirstPersonGameMode.RemoveEnemies` (`self.As BP First Person Game Mode`))
    (`self.K2_DestroyActor`)))

(event `DropWeapon`)

(event `self.Sphere.OnComponentBeginOverlap`
  (params (OverlappedComponent :type "PrimitiveComponent Object Reference") (OtherActor :type "Actor Object Reference") (OtherComp :type "PrimitiveComponent Object Reference") (OtherBodyIndex :type Integer) (bFromSweep :type Boolean) (SweepResult :type "HitResult Structure (by ref)"))
  (if (== OtherActor (`GameplayStatics.GetPlayerPawn` 0))
    (set `self.OnEnemy?` true)
    (if (not (`self.AttackInCooldown?`))
      (`self.DamagePlayer`))))

(event `self.Sphere.OnComponentEndOverlap`
  (params (OverlappedComponent :type "PrimitiveComponent Object Reference") (OtherActor :type "Actor Object Reference") (OtherComp :type "PrimitiveComponent Object Reference") (OtherBodyIndex :type Integer))
  (if (== (`GameplayStatics.GetPlayerPawn` 0) OtherActor)
    (set `self.OnEnemy?` false)))

(event `DamagePlayer`
  (if (and (not (`self.AttackInCooldown?`)) (`self.OnEnemy?`))
    (`/Game/Blueprints/BP_FirstPersonCharacter.DamageTaken` (`self.MainCharather`) (`self.Damage`))
    (set `self.AttackInCooldown?` true)
    (`KismetSystemLibrary.Delay` (`self.AttackSpeed`))
    (set `self.AttackInCooldown?` false)
    (`self.DamagePlayer`)))

(fn `UserConstructionScript`)