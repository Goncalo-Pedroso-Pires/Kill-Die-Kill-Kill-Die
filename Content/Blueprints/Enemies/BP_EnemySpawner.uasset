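; Destructible enemy spawner that registers with BP_FirstPersonGameMode and periodically releases waves of enemies around itself.
; After a start delay it spawns an initial wave, then Spawn and the delayed SpawnEnemies event call each other to repeat.
; Each enemy lands on a random nearby navigable point, with a chance roll choosing between rare and swarm classes.
; DamageTaken reduces health; at zero the spawner unregisters, plays a death sound and destroys itself.
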(event `self.ReceiveBeginPlay`
  (`|ExecutionSequence`
    (:`then_0`
      (set `self.Health` (`self.MaxHealth`))
      (bind _asbp_first_person_game_mode (cast `/Game/FirstPerson/Blueprints/BP_FirstPersonGameMode` (`GameplayStatics.GetGameMode`)))
      (bind _output_get (set `self.GameMode` _asbp_first_person_game_mode))
      (`/Game/FirstPerson/Blueprints/BP_FirstPersonGameMode.AddSpawners` _output_get self))
    (:`then_1`
      (`KismetSystemLibrary.Delay` (`self.StartSpawn`))
      (`GameplayStatics.PlaySoundAtLocation` "/Game/Audio/SFX/Sound_effects/Spawner/SpawnerSPAWN.SpawnerSPAWN" (`SceneComponent.K2_GetComponentLocation` (`self.StaticMesh`)) (struct) 1.0 1.0 0.0 null null null null)
      (`self.Spawn` (- (`self.StartNumberOfEnemies`) 1)))))

(event `SpawnEnemies`
  (`KismetSystemLibrary.Delay` (`self.SpawnInterval`))
  (`GameplayStatics.PlaySoundAtLocation` "/Game/Audio/SFX/Sound_effects/Spawner/SpawnerSPAWN.SpawnerSPAWN" (`SceneComponent.K2_GetComponentLocation` (`self.StaticMesh`)) (struct) 1.0 1.0 0.0 null null null null)
  (`self.Spawn` (- (`self.Spawns`) 1)))

(event `/Game/Blueprints/Enemies/Damageable.DamageTaken`
  (params (Damage :type "Float (double-precision)"))
  (bind _output_get (set `self.Health` (- (`self.Health`) Damage)))
  (if (<= _output_get 0.0)
    (`/Game/FirstPerson/Blueprints/BP_FirstPersonGameMode.Remove Spawner` (`self.GameMode`) self)
    (`GameplayStatics.PlaySoundAtLocation` "/Game/Audio/SFX/Sound_effects/Spawner/SpawnerDEATH.SpawnerDEATH" (`SceneComponent.K2_GetComponentLocation` (`self.StaticMesh`)) (struct) 1.0 1.0 0.0 null null null null)
    (`self.K2_DestroyActor`)))

(fn `UserConstructionScript`)